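; BP_BulletCharacter is a shooter player character that handles its gun setup, aim zoom, crosshair and firing effects.
; On BeginPlay the server spawns a pistol, attaching its body, slider and magazine to separate components and applying the gun's arm mesh and AnimBP.
; The local player gets a HUD whose crosshair spread follows velocity each Tick.
; Events drive timeline FOV zoom when aiming, plus muzzle flash, brief light and short-lived ejected casing.
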(event EventBeginPlay
  (Utilities|FlowControl|Sequence
    (:then_0
      (if (Networking|IsServer)
        (CallFunction|SpawnGun "/Game/Blueprints/Weapons/Pistol/BP_Pistol.BP_Pistol_C")))
    (:then_1
      (if (Pawn|IsLocallyControlled)
        (bind _returnvalue (UserInterface|CreateWidget "/Game/UI/UMG_PlayerHUD.UMG_PlayerHUD_C"))
        (Variables|Default|SetCrosshair (Variables|/Game/UI/UMG_PlayerHUD.UMG_PlayerHUD_C|GetUMG_Crosshair _returnvalue))
        (UserInterface|Viewport|AddtoViewport _returnvalue 0)))))

(event EventCameraFovLerp
  (if (Variables|Default|GetbIsAiming)
    (bind _camerafov (Timeline|CameraFov Play)
      (:Update
        (Camera|SetFieldOfView (Variables|Default|Getcam) _camerafov)))
    (else
      (Timeline|CameraFov Reverse))))

(event EventTick
  (params (DeltaSeconds :type Float%20%28single-precision%29))
  (Variables|/Game/UI/UMG_Crosshair.UMG_Crosshair_C|Setcrosshair_spread (Variables|Default|GetCrosshair) (Math|Float|MapRangeClamped (Math|Vector|VectorLength (Transformation|GetVelocity)) 0.0 4.5e+02 5.0 8e+01)))

(event EventPlayMuzzleFlash
  (bind _muzzleflashposition (Variables|Default|GetMuzzleFlashPosition))
  (Utilities|FlowControl|Sequence
    (:then_0
      (Effects|SpawnEmitterAttached "/Game/ParticleSystems/PS_Muzzle_Flash.PS_Muzzle_Flash" _muzzleflashposition "None" (Transformation|GetWorldLocation _muzzleflashposition) (Transformation|GetWorldRotation _muzzleflashposition) "1.000000,1.000000,1.000000" "KeepWorldPosition")
      (Rendering|SetVisibility (Variables|Default|GetMuzzleFlashLight) true false)
      (Utilities|FlowControl|Delay 0.05)
      (Rendering|SetVisibility (Variables|Default|GetMuzzleFlashLight) false false))
    (:then_1
      (bind _returnvalue (Game|SpawnActorfromClass "/Game/Blueprints/Weapons/Pistol/BP_Casing.BP_Casing_C" (Transformation|GetWorldTransform (Variables|Default|GetCasingSpawnPoint)) "AlwaysSpawn" 0 0))
      (Transformation|SetActorRotation _returnvalue (Math|Random|RandomRotator true))
      (Physics|AddImpulse (Variables|/Game/Blueprints/Weapons/Pistol/BP_Casing.BP_Casing_C|GetCasing _returnvalue) (* (Math|Vector|GetForwardVector (Transformation|GetWorldRotation (Variables|/Game/Blueprints/Weapons/Pistol/BP_Casing.BP_Casing_C|GetCasing _returnvalue))) (Math|Random|RandomFloatinRange 15.0 2e+01)) "None" false)
      (Utilities|FlowControl|Delay 0.1)
      (Actor|DestroyActor _returnvalue))))

(fn ConstructionScript)

(fn SpawnGun
  (params (gunToSpawn :type Base%20Weapon%20Class%20Reference))
  (bind _self self)
  (bind _mesh (Variables|Character|GetMesh))
  (bind _slidercomponents (Variables|Default|GetSliderComponents))
  (bind _magcomponents (Variables|Default|GetMagComponents))
  (bind _gunmaincomponents (Variables|Default|GetGunMainComponents))
  (bind _returnvalue (Game|SpawnActorfromClass gunToSpawn (Math|Transform|MakeTransform "0, 0, 0" "0, 0, 0" "1.000000,1.000000,1.000000") "Undefined" _self _self)) ; Starting Gun
  (bind _output_get (Variables|Default|SetcurrentWeapon _returnvalue))
  (Actor|SetOwner _output_get self)
  (Utilities|FlowControl|Sequence
    (:then_0
      (Transformation|AttachComponentToComponent (Variables|/Script/Bullet.BaseWeapon|GetgunMain (Variables|Default|GetcurrentWeapon)) _gunmaincomponents "None" "KeepRelative" "KeepRelative" "KeepRelative" true)
      (Transformation|SetWorldScale3D _gunmaincomponents "0.050000,0.050000,0.050000")
      (Transformation|SetWorldRotation _gunmaincomponents "0.000000,-90.000000,270.000000" false false))
    (:then_1
      (Transformation|AttachComponentToComponent (Variables|/Script/Bullet.BaseWeapon|Getslider (Variables|Default|GetcurrentWeapon)) _slidercomponents "None" "KeepRelative" "KeepRelative" "KeepRelative" true)
      (Transformation|SetWorldScale3D _slidercomponents "0.050000,0.050000,0.050000")
      (Transformation|SetWorldRotation _slidercomponents "0.000000,-90.000000,270.000000" false false))
    (:then_2
      (Transformation|AttachComponentToComponent (Variables|/Script/Bullet.BaseWeapon|Getmagazine (Variables|Default|GetcurrentWeapon)) _magcomponents "None" "KeepRelative" "KeepRelative" "KeepRelative" true)
      (Transformation|SetWorldScale3D _magcomponents "0.050000,0.050000,0.050000")
      (Transformation|SetWorldRotation _magcomponents "0.000000,-90.000000,270.000000" false false))
    (:then_3
      (Class|SkinnedMeshComponent|SetSkeletalMesh _mesh (Variables|/Script/Bullet.BaseWeapon|GetarmMesh (Variables|Default|GetcurrentWeapon)) true))
    (:then_4
      (Class|SkeletalMeshComponent|SetAnimClass _mesh (Variables|/Script/Bullet.BaseWeapon|GetgunAnimBP (Variables|Default|GetcurrentWeapon))))))